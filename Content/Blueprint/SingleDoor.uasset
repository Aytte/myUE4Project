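; Single swinging door that toggles open and closed when its Box component is hit.
; A locked door compares the player character's held item to Required; a match consumes the item and unlocks without opening.
; The RotateDoor timeline plays or reverses to drive door yaw.
; While open with positive OpenTime, its update starts a padded Delay that calls OpenDoor, re-entering the toggle to close it automatically.
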(event OnComponentHit(Box)
  (params (HitComponent :type Primitive%20Component%20Object%20Reference) (OtherActor :type Actor%20Object%20Reference) (OtherComp :type Primitive%20Component%20Object%20Reference) (NormalImpulse :type Vector :default "0, 0, 0") (Hit :type Hit%20Result%20Structure%20%28by%20ref%29))
  (if (Variables|DoorStatus|GetisLocked)
    (if (Utilities|Enum|Equal(Enum) (Variables|Default|Getrequired) (Variables|/Game/Character/RenewChar.RenewChar_C|GetinHand (Variables|Default|GetChar)))
      (Variables|DoorStatus|SetisLocked false)
      (Development|PrintString "Unlocked")
      (Default|UseItem (Variables|Default|GetChar)))
    (elif (Variables|Default|GetisOpen)
      (Variables|Default|SetisOpen (not (Variables|Default|GetisOpen)))
      (bind _roate (Timeline|RotateDoor Reverse)
        (:Update
          (Transformation|SetRelativeRotation (Variables|Default|GetDoor) (Math|Rotator|MakeRotator 0.0 0.0 _roate) false false)
          (if (and (not (<= (Variables|DoorStatus|GetopenTime) 0.0)) (Variables|Default|GetisOpen))
            (Utilities|FlowControl|Delay (+ (Variables|DoorStatus|GetopenTime) 3.0))
            (if (Variables|Default|GetisOpen)
              (CallFunction|OpenDoor)))))
      (else
        (Variables|Default|SetisOpen (not (Variables|Default|GetisOpen)))
        (Timeline|RotateDoor Play)))))

(event Custom|OpenDoor
  (if (Variables|Default|GetisOpen)
    (Variables|Default|SetisOpen (not (Variables|Default|GetisOpen)))
    (bind _roate (Timeline|RotateDoor Reverse)
      (:Update
        (Transformation|SetRelativeRotation (Variables|Default|GetDoor) (Math|Rotator|MakeRotator 0.0 0.0 _roate) false false)
        (if (and (not (<= (Variables|DoorStatus|GetopenTime) 0.0)) (Variables|Default|GetisOpen))
          (Utilities|FlowControl|Delay (+ (Variables|DoorStatus|GetopenTime) 3.0))
          (if (Variables|Default|GetisOpen)
            (CallFunction|OpenDoor)))))
    (else
      (Variables|Default|SetisOpen (not (Variables|Default|GetisOpen)))
      (Timeline|RotateDoor Play))))

(event EventTick
  (params (DeltaSeconds :type Float%20%28single-precision%29)))

(event EventBeginPlay
  (if (Variables|DoorStatus|GetisLocked)
    (Variables|Default|SetChar (.AsRenew%20Char (Utilities|Casting|CastToRenewChar (Game|GetPlayerCharacter 0))))))

(fn ConstructionScript)